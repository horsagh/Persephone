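; BP_SummonedShield is a cultist enemy's summoned shield actor with its own health and a limited lifetime.
; TakeDamage subtracts from Health and calls Die, which destroys the actor, once Health reaches zero or below.
; A Delay on Tick throttles a fixed self-damage call to about once per second, so the shield decays even when nothing hits it.
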(event `Die`
  (`self.K2_DestroyActor`))

(event `self.TakeDamage`
  (params (Damage :type Integer) (Type :type "/Game/Spirit/E_ManaType Enum" :default "NewEnumerator0") (HitForwardVec :type "Vector Structure"))
  (bind _output_get (set `self.Health` (- (`self.Health`) Damage)))
  (if (<= _output_get 0)
    (`self.Die`)))

(event `self.ReceiveTick`
  (params (DeltaSeconds :type "Float (single-precision)"))
  (`KismetSystemLibrary.Delay` 1.0)
  (`self.TakeDamage` 10))

(fn `UserConstructionScript`)
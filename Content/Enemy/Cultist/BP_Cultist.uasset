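; Cultist enemy that takes damage, ragdolls on death and can summon a shield facing the player.
; Hits deal damage scaled from the previous frame's velocity and the hit normal, printing the value for debugging.
; Lethal damage disables the capsule, enables mesh physics and applies an impulse along the hit direction.
; Basic attack, elemental summons and sight response are empty; the delayed shield-summon and EQS logic is disconnected.
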(event `self.ReceiveBeginPlay`
  (set `self.Targetted Player` (cast `/Game/FirstPerson/Blueprints/BP_FirstPersonCharacter` (`GameplayStatics.GetPlayerCharacter` 0) :!pure true)))

(event `Summon Shield`
  (bind _returnvalue (`self.K2_GetActorLocation`))
  (bind _returnvalue_2 (`|SpawnActorFromClass` "/Game/Enemy/Cultist/BP_SummonedShield.BP_SummonedShield_C" (`KismetMathLibrary.MakeTransform` _returnvalue (`KismetMathLibrary.FindLookAtRotation` _returnvalue (`self.K2_GetActorLocation` (`self.Targetted Player`)))) "Undefined" "OverrideRootScale" null null))
  (set `self.Shield` _returnvalue_2))

(event `Basic Attack`)

(event `/Game/Enemy/BPI_Hittable.TakeDamage`
  (params (Damage :type "Float (double-precision)") (Type :type "/Game/Spirit/E_ManaType Enum" :default "NewEnumerator0") (HitForwardVec :type "Vector Structure"))
  (bind _output_get (set `self.Health` (- (`self.Health`) Damage)))
  (if (<= _output_get 0.0)
    (`self.Die`)
    (`PrimitiveComponent.AddImpulse` (`self.Mesh`) (* (`KismetMathLibrary.Normal` HitForwardVec) 20000.0) "None" false)))

(event `Die`
  (bind _mesh (`self.Mesh`))
  (`PrimitiveComponent.SetCollisionEnabled` _mesh "QueryAndPhysics")
  (`PrimitiveComponent.SetCollisionEnabled` (`self.CapsuleComponent`) "NoCollision")
  (`PrimitiveComponent.SetSimulatePhysics` _mesh true))

(event `Summon Flora`)

(event `Summon Fauna`)

(event `Summon Ferrous`)

(event `Summon Flood`)

(event `self.PawnSensing.OnSeePawn`
  (params (Pawn :type "Pawn Object Reference")))

(event `self.ReceiveHit`
  (params (MyComp :type "PrimitiveComponent Object Reference") (Other :type "Actor Object Reference") (OtherComp :type "PrimitiveComponent Object Reference") (bSelfMoved :type Boolean) (HitLocation :type "Vector Structure") (HitNormal :type "Vector Structure") (NormalImpulse :type "Vector Structure") (Hit :type "HitResult Structure (by ref)"))
  (bind _returnvalue (/ (`KismetMathLibrary.VSize` (* HitNormal (`self.LastFrameVel`))) 15.0))
  (`KismetSystemLibrary.PrintString` (`KismetStringLibrary.Conv_DoubleToString` _returnvalue))
  (`/Game/Enemy/BPI_Hittable.TakeDamage` _returnvalue "NewEnumerator5" HitNormal))

(event `self.ReceiveTick`
  (params (DeltaSeconds :type "Float (single-precision)"))
  (set `self.LastFrameVel` (`self.GetVelocity` self)))

(fn `UserConstructionScript`)
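; BP_MoveableEnemy is an enemy that takes damage and collapses into physics simulation when killed.
; TakeDamage reduces Health only while InvulnerabilityTimer is zero or below, and calls Die once Health runs out.
; Die disables capsule collision and turns on mesh collision and physics, after which TakeDamage launches the body with an impulse along the hit direction.
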(event `/Game/Enemy/BPI_Hittable.TakeDamage`
  (params (Damage :type "Float (double-precision)") (Type :type "/Game/Spirit/E_ManaType Enum" :default "NewEnumerator0") (HitForwardVec :type "Vector Structure"))
  (if (<= (`self.InvulnerabilityTimer`) 0.0)
    (bind _output_get (set `self.Health` (- (`self.Health`) Damage)))
    (if (<= _output_get 0.0)
      (`self.Die`)
      (`PrimitiveComponent.AddImpulse` (`self.Mesh`) (* (`KismetMathLibrary.Normal` HitForwardVec) 20000.0) "None" false))))

(event `Die`
  (bind _mesh (`self.Mesh`))
  (`PrimitiveComponent.SetCollisionEnabled` _mesh "QueryAndPhysics")
  (`PrimitiveComponent.SetCollisionEnabled` (`self.CapsuleComponent`) "NoCollision")
  (`PrimitiveComponent.SetSimulatePhysics` _mesh true))

(fn `UserConstructionScript`)
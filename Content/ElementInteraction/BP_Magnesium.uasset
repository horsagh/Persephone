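; Magnesium element actor that sets off a blinding flash one second after being burned or waterlogged.
; Detonation finds player characters in FlashRadius and traces on Visibility to each camera, flashing only when the line of sight is clear.
; The flash overwrites the settings of the first PostProcessVolume found in the level, then fades through a recursive delayed event with eased interpolation.
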(event `/Game/ElementInteraction/Interfaces/BPI_Waterloggable.Waterlog`
  (`KismetSystemLibrary.Delay` 1.0)
  (`self.Detonate`))

(event `self.ReceiveBeginPlay`
  (bind _outactors (`GameplayStatics.GetAllActorsOfClass` "/Script/Engine.PostProcessVolume"))
  (set `self.Post Process` (`|GetArrayItem` _outactors)))

(event `Detonate`
  (for _array_element (`PrimitiveComponent.GetOverlappingActors` (`self.FlashRadius`) "/Game/FirstPerson/BP_FirstPersonCharacter.BP_FirstPersonCharacter_C")
    (bind (_outhit _returnvalue) (`KismetSystemLibrary.LineTraceSingle` (`SceneComponent.K2_GetComponentLocation` (`self.Sphere`)) (`SceneComponent.K2_GetComponentLocation` (`/Game/FirstPerson/BP_FirstPersonCharacter.FirstPersonCamera` (cast `/Game/FirstPerson/BP_FirstPersonCharacter` _array_element :!pure true))) "TraceTypeQuery1"))
    (if (not _returnvalue)
      (set `self.FlashIntensity` 1.0)
      (set `PostProcessVolume.Settings` (make `PostProcessSettings` :`BloomIntensity` 300.0) (`self.Post Process`))
      (`self.FadeFlash`))))

(event `FadeFlash`
  (bind _flashintensity (`self.FlashIntensity`))
  (set `self.FlashIntensity` (- _flashintensity 0.005))
  (set `PostProcessVolume.Settings` (make `PostProcessSettings` :`BloomIntensity` (`KismetMathLibrary.FInterpEaseInOut` 0.0 300.0 _flashintensity 10.0)) (`self.Post Process`))
  (if (> (`self.FlashIntensity`) 0.0)
    (`KismetSystemLibrary.Delay` 0.02)
    (`self.FadeFlash`)
    (else
      (set `PostProcessVolume.Settings` (make `PostProcessSettings` :`BloomIntensity` 0.0) (`self.Post Process`)))))

(event `/Game/ElementInteraction/Interfaces/BPI_Flammable.Burn`
  (`KismetSystemLibrary.Delay` 1.0)
  (`self.Detonate`))

(fn `UserConstructionScript`)
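; Fireball projectile for the player's Flare ability that explodes on hit or expires after two seconds.
; Explode spawns a Niagara effect, then line-traces to each component in BlastRadius, burning unobscured elementals and damaging hittables, with a bonus for direct hits.
; It knocks back characters, lightly hurts the player, and launches physics objects as damaging projectiles.
; On destruction it passes its location to the casting hand's EndSpecial.
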(event `self.ReceiveBeginPlay`
  (bind _asbp_first_person_character (cast `/Game/Trials/Player/BP_FirstPersonCharacter` (`self.GetInstigator` self))
    (:`then`
      (set `self.Player` _asbp_first_person_character))
    (:`CastFailed`
      (`KismetSystemLibrary.PrintString` "Cast failed - player is not BP_FirstPersonCharacter")))
  (`KismetSystemLibrary.Delay` 2.0)
  (`self.K2_DestroyActor`))

(event `self.ReceiveDestroyed`
  (`/Game/Trials/Player/BP_Hand.EndSpecial` (`self.Casting Hand`) (`self.K2_GetActorLocation`) null))

(event `self.ReceiveHit`
  (params (MyComp :type "PrimitiveComponent Object Reference") (Other :type "Actor Object Reference") (OtherComp :type "PrimitiveComponent Object Reference") (bSelfMoved :type Boolean) (HitLocation :type "Vector Structure") (HitNormal :type "Vector Structure") (NormalImpulse :type "Vector Structure") (Hit :type "HitResult Structure (by ref)"))
  (`self.Explode` Other)
  (`self.K2_DestroyActor`))

(fn `Explode`
  (params (`Direct Hit` :type "Actor Object Reference"))
  (locals (DirectHitActor :type "Actor Object Reference") (ArrayElem :type "SceneComponent Object Reference"))
  (bind _returnvalue (`ActorComponent.GetOwner` (`local.ArrayElem`)))
  (bind _returnvalue_2 (`ActorComponent.GetOwner` (`local.ArrayElem`)))
  (bind _returnvalue_3 (`KismetMathLibrary.Normal` (- (`SceneComponent.K2_GetComponentLocation` (`local.ArrayElem`)) (`self.K2_GetActorLocation`))))
  (bind _returnvalue_4 (* _returnvalue_3 1000.0))
  (`NiagaraFunctionLibrary.SpawnSystemAtLocation` "/Game/AdvancedMagicFX13/Particles/Niagara/NS_ky_explosion3.NS_ky_explosion3" (`self.K2_GetActorLocation`))
  (set `local.DirectHitActor` `Direct Hit`)
  (for _array_element (`PrimitiveComponent.GetOverlappingComponents` (`self.BlastRadius`))
    (set `local.ArrayElem` _array_element)
    (bind (_outhit _returnvalue_5) (`KismetSystemLibrary.LineTraceSingle` (`self.K2_GetActorLocation`) (`SceneComponent.K2_GetComponentLocation` (`local.ArrayElem`)) "TraceTypeQuery4" false (`|MakeArray` _returnvalue_2)))
    (if (not _returnvalue_5)
      (bind _asbpi_elemental (cast `/Game/Trials/EnvironmentBPs/ElementInteraction/Interfaces/BPI_Elemental` _returnvalue_2)
        (:`then`
          (`/Game/Trials/EnvironmentBPs/ElementInteraction/Interfaces/BPI_Elemental.Burn` _asbpi_elemental))
        (:`CastFailed`
          _))
      (switch `EComponentMobility` (`SceneComponent.Mobility` (`local.ArrayElem`))
        (:`Static`
          (if (`KismetSystemLibrary.DoesImplementInterface` _returnvalue "/Game/Trials/Enemies/BPI_Hittable.BPI_Hittable_C") :!label _label
            (message `/Game/Trials/Enemies/BPI_Hittable.TakeDamage` _returnvalue (`KismetMathLibrary.SelectInt` 25 22 (== (`ActorComponent.GetOwner` (`local.ArrayElem`)) (`local.DirectHitActor`))) "NewEnumerator7" _returnvalue_4)))
        (:`Stationary`
          (goto _label))
        (:`Movable`
          (bind _ascharacter (cast `Character` (`ActorComponent.GetOwner` (`local.ArrayElem`)))
            (:`then`
              (`CharacterMovementComponent.AddImpulse` (`Character.CharacterMovement` _ascharacter) _returnvalue_4 true)
              (bind _asbp_first_person_character (cast `/Game/Trials/Player/BP_FirstPersonCharacter` _ascharacter)
                (:`then`
                  (`/Game/Trials/Player/BP_FirstPersonCharacter.TakeDamage` _asbp_first_person_character 2))
                (:`CastFailed`
                  (goto _label))))
            (:`CastFailed`
              (if (`SceneComponent.IsSimulatingPhysics` (`local.ArrayElem`) "None")
                (bind _asprimitive_component (cast `PrimitiveComponent` (`local.ArrayElem`))
                  (:`then`
                    (`PrimitiveComponent.AddImpulseAtLocation` _asprimitive_component (* _returnvalue_3 800000.0) (`self.K2_GetActorLocation`) "None")
                    (`/Game/Trials/Player/BP_FirstPersonCharacter.MakeProjectileDamaging` (`self.Player`) _asprimitive_component)
                    (goto _label))
                  (:`CastFailed`
                    (goto _label)))
                (else
                  (goto _label))))))))))

(fn `UserConstructionScript`)
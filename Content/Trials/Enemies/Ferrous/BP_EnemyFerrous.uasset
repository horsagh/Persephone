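; Ferrous enemy Blueprint that leaves behind a mana spirit when it dies.
; On death it spawns a BP_Spirit at its own transform, assigns it a fixed mana type, then runs the parent death logic.
; A separate proximity helper gathers static mesh components overlapping a given mesh and appends those not already tracked to the floor-is-lava affected floor list.
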(event `self.Die`
  (bind (_returnvalue_location _returnvalue_rotation) (`KismetMathLibrary.BreakTransform` (`self.GetTransform`)))
  (bind _returnvalue (`|SpawnActorFromClass` "/Game/Trials/EnvironmentBPs/BP_Spirit.BP_Spirit_C" (`KismetMathLibrary.MakeTransform` _returnvalue_location _returnvalue_rotation) "Undefined" "MultiplyWithRoot" null null))
  (`/Game/Trials/EnvironmentBPs/BP_Spirit.Update Mana Type` _returnvalue "NewEnumerator3")
  (`parent.Die`))

(fn `Use Proximity Tester`
  (params (`Original Mesh` :type "StaticMeshComponent Object Reference"))
  (locals (ComponentsToAdd :type "Array of StaticMeshComponent Object Reference"))
  (for _array_element (`PrimitiveComponent.GetOverlappingComponents` `Original Mesh`)
    (bind _asstatic_mesh_component (cast `StaticMeshComponent` _array_element))
    (if (not (`KismetArrayLibrary.Array_Contains` (`self.FloorIsLavaEffectedFloor`) _asstatic_mesh_component))
      (`KismetArrayLibrary.Array_Add` (`local.ComponentsToAdd`) _asstatic_mesh_component)))
  (`KismetArrayLibrary.Array_Append` (`self.FloorIsLavaEffectedFloor`) (`local.ComponentsToAdd`)))

(fn `UserConstructionScript`
  (`parent.UserConstructionScript`))
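; BP_Dummy is a target dummy enemy that visualizes the hits it receives.
; On TakeDamage, it shows the damage as text and draws a five-second debug arrow along the hit direction, both colored by damage type.
; It then forwards the hit to the parent's TakeDamage, while its own Die and Tick events are left empty.
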(event `/Game/Trials/Enemies/BPI_Hittable.TakeDamage`
  (params (Damage :type Integer) (Type :type "/Game/Trials/EnvironmentBPs/Spirit/E_ManaType Enum" :default "NewEnumerator0") (HitForwardVec :type "Vector Structure"))
  (bind _returnvalue (`self.K2_GetActorLocation`))
  (bind _returnvalue_2 (select `/Game/Trials/EnvironmentBPs/Spirit/E_ManaType` Type :`NewEnumerator0` (struct :`R` 0.007053 :`G` 0.677083 :`B` 0.08377 :`A` 1.0) :`NewEnumerator1` (struct :`R` 0.796875 :`G` 0.40501 :`B` 0.023654 :`A` 1.0) :`NewEnumerator2` (struct :`G` 0.082834 :`B` 0.682292 :`A` 1.0) :`NewEnumerator3` (struct :`R` 0.432292 :`G` 0.432292 :`B` 0.432292 :`A` 1.0) :`NewEnumerator7` (struct :`R` 0.723958 :`G` 0.044405 :`B` 0.030001 :`A` 1.0) :`NewEnumerator6` (struct :`R` 0.2 :`G` 0.6 :`B` 0.7 :`A` 1.0) :`NewEnumerator5` (struct :`R` 0.114435 :`G` 0.114435 :`B` 0.114435 :`A` 1.0) :!type "LinearColor Structure"))
  (`TextRenderComponent.K2_SetText` (`self.TextRender_0`) (`KismetTextLibrary.Conv_IntToText` Damage))
  (`TextRenderComponent.SetTextRenderColor` (`self.TextRender_0`) (`KismetMathLibrary.Conv_LinearColorToColor` _returnvalue_2))
  (`KismetSystemLibrary.DrawDebugArrow` _returnvalue (+ _returnvalue (* (`KismetMathLibrary.Normal` HitForwardVec 0.1) 150.0)) 10.0 _returnvalue_2 5.0 2.0)
  (`parent.TakeDamage` Damage Type HitForwardVec))

(event `self.Die`)

(event `self.ReceiveTick`
  (params (DeltaSeconds :type "Float (single-precision)")))

(fn `UserConstructionScript`)
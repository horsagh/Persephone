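; BP_EnemyProjectile is an enemy projectile that damages the first-person player on impact.
; On spawn it launches its Sphere forward with a physics impulse, then blocks the Pawn channel after a short delay.
; A hit on the player outside the MeleeBox applies damage and destroys the projectile, while MeleeBox hits do neither.
; Hits on anything else destroy it, except hits on its Instigator.
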(event `self.ReceiveBeginPlay`
  (`PrimitiveComponent.AddImpulse` (`self.Sphere`) (* (`self.GetActorForwardVector`) 100000.0) "None" false)
  (`KismetSystemLibrary.Delay` 0.2)
  (`PrimitiveComponent.SetCollisionResponseToChannel` (`self.Sphere`) "ECC_Pawn" "ECR_Block"))

(event `self.Sphere.OnComponentHit`
  (params (HitComponent :type "PrimitiveComponent Object Reference") (OtherActor :type "Actor Object Reference") (OtherComp :type "PrimitiveComponent Object Reference") (NormalImpulse :type "Vector Structure") (Hit :type "HitResult Structure (by ref)"))
  (bind _asbp_first_person_character (cast `/Game/Trials/Player/BP_FirstPersonCharacter` OtherActor)
    (:`then`
      (if (not (== OtherComp (`/Game/Trials/Player/BP_FirstPersonCharacter.MeleeBox` _asbp_first_person_character)))
        (`/Game/Trials/Player/BP_FirstPersonCharacter.TakeDamage` _asbp_first_person_character 2)
        (`self.K2_DestroyActor` :!label _label)))
    (:`CastFailed`
      (if (not (== OtherActor (`self.Instigator`)))
        (goto _label)))))

(fn `UserConstructionScript`)
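; Flood-type enemy that moves straight at perceived players without pathfinding and self-destructs when one comes close.
; Entering its detonation radius swaps a material and starts a one-second fuse; the explosion damages and knocks back players with an unblocked line trace, then destroys the actor.
; Incoming damage is scaled by elemental type before reaching the parent class.
; Death spawns a spirit set to Flood mana.
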(event `/Game/Trials/Enemies/BPI_Hittable.TakeDamage`
  (params (Damage :type Integer) (Type :type "/Game/Trials/EnvironmentBPs/Spirit/E_ManaType Enum" :default "NewEnumerator0") (HitForwardVec :type "Vector Structure"))
  (`parent.TakeDamage` (* Damage (select `/Game/Trials/EnvironmentBPs/Spirit/E_ManaType` Type :`NewEnumerator0` 1.5 :`NewEnumerator1` 1.0 :`NewEnumerator2` 0.7 :`NewEnumerator3` 1.0 :`NewEnumerator7` 0.7 :`NewEnumerator6` 1.0 :`NewEnumerator5` 1.0)) Type HitForwardVec))

(event `self.AIPerception.OnPerceptionUpdated`
  (params (UpdatedActors :type "Array of Actor Object Reference (by ref)"))
  (for _array_element UpdatedActors
    (bind _asbp_first_person_character (cast `/Game/Trials/Player/BP_FirstPersonCharacter` _array_element))
    (`AIController.MoveToActor` (`AIBlueprintHelperLibrary.GetAIController` self) _asbp_first_person_character 10.0 true false true null true)))

(event `self.DetonationRadius.OnComponentBeginOverlap`
  (params (OverlappedComponent :type "PrimitiveComponent Object Reference") (OtherActor :type "Actor Object Reference") (OtherComp :type "PrimitiveComponent Object Reference") (OtherBodyIndex :type Integer) (bFromSweep :type Boolean) (SweepResult :type "HitResult Structure (by ref)"))
  (cast `/Game/Trials/Player/BP_FirstPersonCharacter` OtherActor)
  (`PrimitiveComponent.SetMaterial` (`self.Mesh`) 1 "/Game/Trials/EnvironmentBPs/Spirit/Materials/M_Flood.M_Flood")
  (`KismetSystemLibrary.Delay` 1.0)
  (`self.Explode`))

(event `Explode`
  (bind _returnvalue (`self.K2_GetActorLocation`))
  (if (not (`self.Dead`))
    (for _array_element (`PrimitiveComponent.GetOverlappingActors` (`self.DetonationRadius`) "/Game/Trials/Player/BP_FirstPersonCharacter.BP_FirstPersonCharacter_C")
      (bind _asbp_first_person_character (cast `/Game/Trials/Player/BP_FirstPersonCharacter` _array_element))
      (bind _returnvalue_2 (`self.K2_GetActorLocation` _array_element))
      (bind (_outhit _returnvalue_3) (`KismetSystemLibrary.LineTraceSingle` _returnvalue _returnvalue_2 "TraceTypeQuery1"))
      (if (not _returnvalue_3)
        (`CharacterMovementComponent.AddImpulse` (`Character.CharacterMovement` _asbp_first_person_character) (* (`KismetMathLibrary.Normal` (- _returnvalue_2 _returnvalue)) 150000.0) false)
        (`/Game/Trials/Player/BP_FirstPersonCharacter.TakeDamage` _asbp_first_person_character (`self.Damage`))))
    (`self.K2_DestroyActor`)))

(event `self.Die`
  (bind (_returnvalue_location _returnvalue_rotation) (`KismetMathLibrary.BreakTransform` (`self.GetTransform`)))
  (bind _returnvalue (`|SpawnActorFromClass` "/Game/Trials/EnvironmentBPs/BP_Spirit.BP_Spirit_C" (`KismetMathLibrary.MakeTransform` _returnvalue_location _returnvalue_rotation) "Undefined" "MultiplyWithRoot" null null))
  (`/Game/Trials/EnvironmentBPs/BP_Spirit.Update Mana Type` _returnvalue "NewEnumerator2")
  (`parent.Die`))

(fn `UserConstructionScript`
  (`parent.UserConstructionScript`))
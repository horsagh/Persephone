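; BP_Cultist is an enemy Blueprint, apparently an unfinished summoner, that extends its parent's BeginPlay and Tick.
; It caches the first-person player, and SummonShield spawns and stores a BP_SummonedShield rotated toward them.
; Flora, Fauna, Ferrous and Flood summons are empty stubs.
; Tick counts down an invulnerability timer, while the sight-triggered shield respawn, impact damage and timer reset are disconnected and never run.
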(event `self.ReceiveBeginPlay`
  (set `self.Targetted Player` (cast `/Game/Trials/Player/BP_FirstPersonCharacter` (`GameplayStatics.GetPlayerCharacter` 0) :!pure true))
  (`parent.ReceiveBeginPlay`))

(event `Summon Shield`
  (bind _returnvalue (`self.K2_GetActorLocation`))
  (bind _returnvalue_2 (`|SpawnActorFromClass` "/Game/Trials/Enemies/Cultist/BP_SummonedShield.BP_SummonedShield_C" (`KismetMathLibrary.MakeTransform` _returnvalue (`KismetMathLibrary.FindLookAtRotation` _returnvalue (`self.K2_GetActorLocation` (`self.Targetted Player`)))) "Undefined" "OverrideRootScale" null null))
  (set `self.Shield` _returnvalue_2))

(event `Summon Flora`)

(event `Summon Fauna`)

(event `Summon Ferrous`)

(event `Summon Flood`)

(event `self.PawnSensing.OnSeePawn`
  (params (Pawn :type "Pawn Object Reference")))

(event `self.ReceiveHit`
  (params (MyComp :type "PrimitiveComponent Object Reference") (Other :type "Actor Object Reference") (OtherComp :type "PrimitiveComponent Object Reference") (bSelfMoved :type Boolean) (HitLocation :type "Vector Structure") (HitNormal :type "Vector Structure") (NormalImpulse :type "Vector Structure") (Hit :type "HitResult Structure (by ref)")))

(event `self.ReceiveTick`
  (params (DeltaSeconds :type "Float (single-precision)"))
  (bind _invulnerabilitytimer_0 (`self.InvulnerabilityTimer_0`))
  (`parent.ReceiveTick` DeltaSeconds)
  (if (> _invulnerabilitytimer_0 0.0)
    (set `self.InvulnerabilityTimer_0` (- _invulnerabilitytimer_0 DeltaSeconds))))

(fn `UserConstructionScript`)
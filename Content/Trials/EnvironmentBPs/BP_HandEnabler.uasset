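; BP_HandEnabler is a world pickup that unlocks the player's left or right hand, chosen by IsRightHand.
; On overlap it registers itself as the first-person character's Zone and shows an RMB or LMB prompt, which turns toward that player's camera each tick.
; Its Pickup event fires the PickedUp dispatcher, enables the matching hand, refreshes that hand's mana UI and destroys the actor.
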(event `self.ReceiveActorBeginOverlap`
  (params (OtherActor :type "Actor Object Reference"))
  (bind _asbp_first_person_character (cast `/Game/Trials/Player/BP_FirstPersonCharacter` OtherActor))
  (set `/Game/Trials/Player/BP_FirstPersonCharacter.Zone` self _asbp_first_person_character)
  (set `self.OverlappingCharacter` _asbp_first_person_character)
  (`TextRenderComponent.K2_SetText` (`self.TextRender`) (select `bool` (`self.isRightHand`) :`false` "Press LMB to pick up" :`true` "Press RMB to pick up" :!type "Text")))

(event `self.ReceiveActorEndOverlap`
  (params (OtherActor :type "Actor Object Reference"))
  (bind _asbp_first_person_character (cast `/Game/Trials/Player/BP_FirstPersonCharacter` OtherActor))
  (set `/Game/Trials/Player/BP_FirstPersonCharacter.Zone` null _asbp_first_person_character)
  (`TextRenderComponent.K2_SetText` (`self.TextRender`) ""))

(event `Pickup`
  (params (Character :type "/Game/Trials/Player/BP_FirstPersonCharacter Object Reference"))
  (bind _returnvalue (select `bool` (`self.isRightHand`) :`false` (`/Game/Trials/Player/BP_FirstPersonCharacter.LeftHand` Character) :`true` (`/Game/Trials/Player/BP_FirstPersonCharacter.RightHand` Character)))
  (`self.PickedUp`)
  (set `/Game/Trials/Player/BP_Hand.isEnabled` true _returnvalue)
  (`/Game/Trials/Player/BP_Hand.UpdateManaUI` _returnvalue)
  (`self.K2_DestroyActor`))

(event `self.ReceiveTick`
  (params (DeltaSeconds :type "Float (single-precision)"))
  (bind _overlappingcharacter (`self.OverlappingCharacter`))
  (`/Engine/EditorBlueprintResources/StandardMacros.IsValid` _overlappingcharacter
    (:`Is Valid`
      (`SceneComponent.K2_SetWorldRotation` (`self.TextRender`) (`KismetMathLibrary.FindLookAtRotation` (`SceneComponent.K2_GetComponentLocation` (`self.TextRender`)) (`SceneComponent.K2_GetComponentLocation` (`/Game/Trials/Player/BP_FirstPersonCharacter.FirstPersonCamera` _overlappingcharacter))) false false))))

(fn `UserConstructionScript`)
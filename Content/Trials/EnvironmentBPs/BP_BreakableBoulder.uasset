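; Breakable boulder for trial environments that shatters into smaller BP_Boulder actors the first time it takes damage.
; TakeDamage disables collision on the BigBoulder component, then a loop spawns the pieces at random offsets around the actor's location, adjusting for overlaps but always spawning.
; The original actor then destroys itself, with no health or damage threshold check.
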(event `/Game/Trials/Enemies/BPI_Hittable.TakeDamage`
  (params (Damage :type Integer) (Type :type "/Game/Trials/EnvironmentBPs/Spirit/E_ManaType Enum" :default "NewEnumerator0") (HitForwardVec :type "Vector Structure"))
  (`PrimitiveComponent.SetCollisionEnabled` (`self.BigBoulder`) "NoCollision")
  (for _ (range 10)
    (`|SpawnActorFromClass` "/Game/Trials/EnvironmentBPs/BP_Boulder.BP_Boulder_C" (`KismetMathLibrary.Conv_VectorToTransform` (+ (`self.K2_GetActorLocation`) (* (`KismetMathLibrary.RandomUnitVector`) (`KismetMathLibrary.RandomFloatInRange` 0.0 70.0)))) "AdjustIfPossibleButAlwaysSpawn" "MultiplyWithRoot" null null))
  (`self.K2_DestroyActor`))

(fn `UserConstructionScript`)
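; BP_KillOpenedDoor is a double door that opens once every enemy in its Enemies list is dead.
; Tick prunes dead or invalid enemies from the list while the door is closed and calls Open when the list is empty.
; Open sets IsOpen, halting further checks, and uses MoveComponentTo to swing the left and right leaves outward in opposite yaw directions.
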(event `Open`
  (bind _doorr (`self.DoorR`))
  (bind _doorl (`self.DoorL`))
  (set `self.isOpen` true)
  (`|ExecutionSequence`
    (:`then_0`
      (`KismetSystemLibrary.MoveComponentTo` _doorl (`SceneComponent.RelativeLocation` _doorl) (struct :`Yaw` -100.0)))
    (:`then_1`
      (`KismetSystemLibrary.MoveComponentTo` _doorr (`SceneComponent.RelativeLocation` _doorr) (struct :`Yaw` 100.0)))))

(event `self.ReceiveTick`
  (params (DeltaSeconds :type "Float (single-precision)"))
  (bind _enemies (`self.Enemies`))
  (if (`self.isOpen`)
    _
    (elif (< (`KismetArrayLibrary.Array_Length` _enemies) 1)
      (`self.Open`)
      (else
        (for _array_element _enemies
          (`/Engine/EditorBlueprintResources/StandardMacros.IsValid` _array_element
            (:`Is Valid`
              (if (`/Game/Trials/Enemies/BP_MoveableEnemy.Dead` _array_element)
                (`KismetArrayLibrary.Array_RemoveItem` (`self.Enemies`) _array_element :!label _label)))
            (:`Is Not Valid`
              (goto _label))))))))

(fn `UserConstructionScript`)
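; BP_Boulder is an environment blueprint for a boulder with an elemental state, exposed through GetElementalState.
; Its Burn, Freeze, Waterlog, DelayedExplosion and SpawnMagnesium events are empty, leaving all reaction logic unwired.
; The orphaned nodes switch between Default, Molten, Frozen and Waterlogged, with some transitions calling explosion or magnesium events.
; Other orphaned chains print debug explosion text, or swap the mesh for physics, spawn BP_Magnesium and trigger an FS_MasterField.
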(event `self.ReceiveTick`
  (params (DeltaSeconds :type "Float (single-precision)")))

(event `Spawn Magnesium`)

(event `/Game/Trials/EnvironmentBPs/ElementInteraction/Interfaces/BPI_Elemental.Burn`)

(event `/Game/Trials/EnvironmentBPs/ElementInteraction/Interfaces/BPI_Elemental.Freeze`)

(event `Delayed Explosion`)

(event `/Game/Trials/EnvironmentBPs/ElementInteraction/Interfaces/BPI_Elemental.Waterlog`)

(fn `GetElementalState`
  (returns (ElementalState :type "/Game/Trials/EnvironmentBPs/ElementInteraction/Interfaces/E_ElementalState Enum"))
  (return (`self.ElementalState`)))

(fn `UserConstructionScript`)
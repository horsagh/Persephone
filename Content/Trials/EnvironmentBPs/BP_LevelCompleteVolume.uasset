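; BP_LevelCompleteVolume is a trigger actor that ends the level when the first-person character overlaps it.
; It passes its NextLevel to the character's UI, shows the blackout, a "Well Played!" message with the game mode's run time, and a button.
; It then switches input to UI only with the mouse cursor shown and pauses the game.
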(event `self.ReceiveActorBeginOverlap`
  (params (OtherActor :type "Actor Object Reference"))
  (bind _returnvalue (`GameplayStatics.GetPlayerController` 0))
  (bind _asbp_first_person_character (cast `/Game/Trials/Player/BP_FirstPersonCharacter` OtherActor))
  (bind _asbp_first_person_game_mode (cast `/Game/Trials/Player/BP_FirstPersonGameMode` (`GameplayStatics.GetGameMode`)))
  (bind _ui (`/Game/Trials/Player/BP_FirstPersonCharacter.UI` _asbp_first_person_character))
  (set `/Game/Trials/Player/WBP_FirstPerson.NextLevel` (`self.NextLevel`) _ui)
  (`Widget.SetVisibility` (`/Game/Trials/Player/WBP_FirstPerson.Blackout` _ui) "Visible")
  (`/Game/Trials/Player/WBP_FirstPerson.ShowText` _ui "Well Played!" (`KismetStringLibrary.Concat_StrStr` " \nTime: " (`KismetTextLibrary.Conv_TextToString` (`KismetTextLibrary.AsTimespan_Timespan` (`/Game/Trials/Player/BP_FirstPersonGameMode.RunTime` _asbp_first_person_game_mode)))) 1000.0)
  (`Widget.SetVisibility` (`/Game/Trials/Player/WBP_FirstPerson.Button_0` _ui) "Visible")
  (`WidgetBlueprintLibrary.SetInputMode_UIOnlyEx` _returnvalue _ui)
  (set `PlayerController.bShowMouseCursor` true _returnvalue)
  (`GameplayStatics.SetGamePaused` true))

(fn `UserConstructionScript`)
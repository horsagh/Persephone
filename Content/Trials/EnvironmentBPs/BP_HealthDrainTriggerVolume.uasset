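; BP_HealthDrainTriggerVolume is a box trigger volume that changes how fast the first-person character's health drains.
; Begin and end overlap events cast the overlapping actor to BP_FirstPersonCharacter and overwrite its HealthDrainRate with separate enter and exit values.
; TriggerOnEnter and TriggerOnExit switch each side on or off independently, and the previous rate is not saved.
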(event `self.Box.OnComponentEndOverlap`
  (params (OverlappedComponent :type "PrimitiveComponent Object Reference") (OtherActor :type "Actor Object Reference") (OtherComp :type "PrimitiveComponent Object Reference") (OtherBodyIndex :type Integer))
  (bind _asbp_first_person_character (cast `/Game/Trials/Player/BP_FirstPersonCharacter` OtherActor))
  (if (`self.TriggerOnExit`)
    (set `/Game/Trials/Player/BP_FirstPersonCharacter.HealthDrainRate` (`self.HealthDrainRateExit`) _asbp_first_person_character)))

(event `self.Box.OnComponentBeginOverlap`
  (params (OverlappedComponent :type "PrimitiveComponent Object Reference") (OtherActor :type "Actor Object Reference") (OtherComp :type "PrimitiveComponent Object Reference") (OtherBodyIndex :type Integer) (bFromSweep :type Boolean) (SweepResult :type "HitResult Structure (by ref)"))
  (bind _asbp_first_person_character (cast `/Game/Trials/Player/BP_FirstPersonCharacter` OtherActor))
  (if (`self.TriggerOnEnter`)
    (set `/Game/Trials/Player/BP_FirstPersonCharacter.HealthDrainRate` (`self.HealthDrainRateEnter`) _asbp_first_person_character)))

(fn `UserConstructionScript`)
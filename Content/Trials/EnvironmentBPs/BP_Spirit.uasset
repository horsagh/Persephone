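; BP_Spirit is a harvestable mana spirit character whose elemental type sets its sphere material.
; Harvesting stops it, spawns a type-colored Niagara burst and twinkle sound, then hides it without collision at world origin.
; When used, it teleports home and reappears after a delay.
; Using it on a BPI_SpiritContainer instead moves its home there and registers the spirit with it; an AI walk-home path is left unconnected.
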(event `Update Mana Type`
  (params (`New ManaType` :type "/Game/Trials/EnvironmentBPs/Spirit/E_ManaType Enum" :default "NewEnumerator0"))
  (bind _output_get (set `self.ManaType` `New ManaType`))
  (`PrimitiveComponent.SetMaterial` (`self.Sphere`) 0 (select `/Game/Trials/EnvironmentBPs/Spirit/E_ManaType` _output_get :`NewEnumerator0` "/Game/Trials/EnvironmentBPs/Spirit/Materials/MI_Flora.MI_Flora" :`NewEnumerator1` "/Game/Trials/EnvironmentBPs/Spirit/Materials/MI_Fauna.MI_Fauna" :`NewEnumerator2` "/Game/Trials/EnvironmentBPs/Spirit/Materials/M_Flood.M_Flood" :`NewEnumerator3` "/Game/Trials/EnvironmentBPs/Spirit/Materials/MI_Ferrous.MI_Ferrous" :`NewEnumerator7` "/Game/Trials/EnvironmentBPs/Spirit/Materials/M_Flare.M_Flare" :`NewEnumerator6` "/Game/Trials/EnvironmentBPs/Spirit/Materials/M_Frost.M_Frost" :!type "MaterialInterface Object Reference")))

(event `self.ReceiveBeginPlay`
  (`PrimitiveComponent.SetMaterial` (`self.Sphere`) 0 (select `/Game/Trials/EnvironmentBPs/Spirit/E_ManaType` (`self.ManaType`) :`NewEnumerator0` "/Game/Trials/EnvironmentBPs/Spirit/Materials/MI_Flora.MI_Flora" :`NewEnumerator1` "/Game/Trials/EnvironmentBPs/Spirit/Materials/MI_Fauna.MI_Fauna" :`NewEnumerator2` "/Game/Trials/EnvironmentBPs/Spirit/Materials/M_Flood.M_Flood" :`NewEnumerator3` "/Game/Trials/EnvironmentBPs/Spirit/Materials/MI_Ferrous.MI_Ferrous" :`NewEnumerator7` "/Game/Trials/EnvironmentBPs/Spirit/Materials/M_Flare.M_Flare" :`NewEnumerator6` "/Game/Trials/EnvironmentBPs/Spirit/Materials/M_Frost.M_Frost" :!type "MaterialInterface Object Reference"))
  (set `self.Home` (`self.K2_GetActorLocation`))
  (set `self.Uses` 1))

(event `Used`
  (params (NewLocation :type "Vector Structure"))
  (set `self.Uses` 1)
  (set `self.State` "NewEnumerator2")
  (`self.Return`))

(event `Return`
  (`self.K2_SetActorLocation` (`self.Home`))
  (`KismetSystemLibrary.Delay` 2.5)
  (`PrimitiveComponent.SetCollisionEnabled` (`self.CapsuleComponent`) "QueryAndPhysics")
  (`SceneComponent.SetVisibility` (`self.CapsuleComponent`) true true)
  (`KismetSystemLibrary.Delay` 0.1)
  (set `self.State` "NewEnumerator0"))

(event `UsedContainer`
  (params (Container :type "Actor Object Reference"))
  (bind _returnvalue (`self.K2_GetActorLocation` Container))
  (bind _asbpi_spirit_container (cast `/Game/Trials/EnvironmentBPs/Spirit/BPI_SpiritContainer` Container)
    (:`then`
      (set `self.Home` _returnvalue)
      (set `self.Uses` 1)
      (set `self.State` "NewEnumerator2")
      (`/Game/Trials/EnvironmentBPs/Spirit/BPI_SpiritContainer.SetSpirit` _asbpi_spirit_container self)
      (`KismetSystemLibrary.Delay` 2.5)
      (set `self.State` "NewEnumerator0"))
    (:`CastFailed`
      (`self.Used` _returnvalue))))

(event `Harvested`
  (`self.Harvest`)
  (set `self.State` "NewEnumerator1")
  (`MovementComponent.StopMovementImmediately` (`self.CharacterMovement`))
  (`PrimitiveComponent.SetCollisionEnabled` (`self.CapsuleComponent`) "NoCollision")
  (bind _returnvalue (`NiagaraFunctionLibrary.SpawnSystemAtLocation` "/Game/AdvancedMagicFX13/Particles/Niagara/NS_ky_hit_slash.NS_ky_hit_slash" (`self.K2_GetActorLocation`) (struct) (0.3 0.3 0.3)))
  (`GameplayStatics.SpawnSoundAtLocation` "/Game/Trials/Assets/Audio/SW_Twinkle.SW_Twinkle" (`self.K2_GetActorLocation`) (struct) 1.0 1.0 0.0 null null)
  (`NiagaraComponent.SetVariableVec3` _returnvalue "Color" (select `/Game/Trials/EnvironmentBPs/Spirit/E_ManaType` (`self.ManaType`) :`NewEnumerator0` (0.0 255.0 0.0) :`NewEnumerator1` (120.0 60.0 0.0) :`NewEnumerator2` (0.0 0.0 255.0) :`NewEnumerator3` (128.0 128.0 128.0) :`NewEnumerator7` (255.0 0.0 0.0) :`NewEnumerator6` (40.0 140.0 160.0) :`NewEnumerator5` (255.0 255.0 255.0) :!type "Vector Structure"))
  (`SceneComponent.SetVisibility` (`self.CapsuleComponent`) false true)
  (`self.K2_SetActorLocation` (0.0 0.0 0.0)))

(fn `UserConstructionScript`)
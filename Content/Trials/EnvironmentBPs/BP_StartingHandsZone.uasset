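; BP_StartingHandsZone is a trial environment zone that sets the player's starting hand abilities and speedrun timer display.
; On its first Tick it finds overlapping first-person characters, since overlaps are not yet registered at BeginPlay.
; For each, it enables or disables the right and left hands from its flags, refreshes their mana UI, and shows or hides the speedrun timer background.
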(event `self.ReceiveTick`
  (params (DeltaSeconds :type "Float (single-precision)"))
  (if (not (`self.hasFired`))
    (set `self.hasFired` true)
    (for _array_element (`self.GetOverlappingActors` "/Game/Trials/Player/BP_FirstPersonCharacter.BP_FirstPersonCharacter_C")
      (bind _asbp_first_person_character (cast `/Game/Trials/Player/BP_FirstPersonCharacter` _array_element))
      (`|ExecutionSequence`
        (:`then_0`
          (bind _righthand (`/Game/Trials/Player/BP_FirstPersonCharacter.RightHand` _asbp_first_person_character))
          (set `/Game/Trials/Player/BP_Hand.isEnabled` (`self.RightHandEnabled`) _righthand)
          (`/Game/Trials/Player/BP_Hand.UpdateManaUI` _righthand))
        (:`then_1`
          (bind _lefthand (`/Game/Trials/Player/BP_FirstPersonCharacter.LeftHand` _asbp_first_person_character))
          (set `/Game/Trials/Player/BP_Hand.isEnabled` (`self.LeftHandEnabled`) _lefthand)
          (`/Game/Trials/Player/BP_Hand.UpdateManaUI` _lefthand))
        (:`then_2`
          (set `Widget.Visibility` (select `bool` (`self.TimerEnabled`) :`false` "Hidden" :`true` "Visible" :!type "ESlateVisibility Enum") (`/Game/Trials/Player/WBP_FirstPerson.SpeedrunTimeBG` (`/Game/Trials/Player/BP_FirstPersonCharacter.UI` _asbp_first_person_character))))))))

(fn `UserConstructionScript`)
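; BP_TextTriggerVolume is a trigger actor that shows a titled text message on the player's UI when the first-person character overlaps it.
; Overlap calls a TriggerText dispatcher, which ShowText binds to on BeginPlay.
; ShowText passes the title, body and duration to the UI of player 0's character.
; A Retriggerable flag chooses between showing on every overlap or only once, tracked by a Triggered flag.
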(event `self.ReceiveActorBeginOverlap`
  (params (OtherActor :type "Actor Object Reference"))
  (cast `/Game/Trials/Player/BP_FirstPersonCharacter` OtherActor)
  (`self.TriggerText`))

(event `self.ReceiveBeginPlay`
  (add `self.TriggerText` (delegate `ShowText`)))

(event `ShowText`
  (if (`self.Retriggerable`)
    (bind _asbp_first_person_character (cast `/Game/Trials/Player/BP_FirstPersonCharacter` (`GameplayStatics.GetPlayerCharacter` 0) :!label _label))
    (`/Game/Trials/Player/WBP_FirstPerson.ShowText` (`/Game/Trials/Player/BP_FirstPersonCharacter.UI` _asbp_first_person_character) (`self.TextTitle`) (`self.Text`) (`self.Duration`))
    (elif (not (`self.Triggered`))
      (set `self.Triggered` true)
      (goto _label))))

(fn `UserConstructionScript`)
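; BP_Fireball is a fireball ability projectile with a ProjectileMovement component, largely unfinished.
; On BeginPlay it caches its instigator as the player's BP_FirstPersonCharacter, printing an error if the cast fails.
; Tick accumulates time lived, but nothing active reads it.
; The Hit event is empty, and nodes for homing target, distance from initial speed and BlastRadius overlaps are disconnected, so no impact or blast logic runs.
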(event `self.ReceiveBeginPlay`
  (bind _asbp_first_person_character (cast `/Game/FirstPerson/Blueprints/BP_FirstPersonCharacter` (`self.GetInstigator` self))
    (:`then`
      (set `self.Player` _asbp_first_person_character))
    (:`CastFailed`
      (`KismetSystemLibrary.PrintString` "Cast failed - player is not BP_FirstPersonCharacter"))))

(event `self.ReceiveTick`
  (params (DeltaSeconds :type "Float (single-precision)"))
  (bind _output_get (set `self.Time lived` (+ DeltaSeconds (`self.Time lived`)))))

(event `self.ReceiveHit`
  (params (MyComp :type "PrimitiveComponent Object Reference") (Other :type "Actor Object Reference") (OtherComp :type "PrimitiveComponent Object Reference") (bSelfMoved :type Boolean) (HitLocation :type "Vector Structure") (HitNormal :type "Vector Structure") (NormalImpulse :type "Vector Structure") (Hit :type "HitResult Structure (by ref)")))

(fn `UserConstructionScript`)
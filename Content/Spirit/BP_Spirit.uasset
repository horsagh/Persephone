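; BP_Spirit is an AI-moved mana spirit whose sphere material matches its ManaType and whose spawn point becomes Home.
; Harvested stops and hides it with collision off; Used restores it, then after a delay starts Return.
; Return walks it Home via AIMoveTo, with a hidden teleport if a successful move ends too far away, updating State throughout.
; The relocation to Used's NewLocation is disconnected.
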(event `self.ReceiveBeginPlay`
  (`PrimitiveComponent.SetMaterial` (`self.Sphere`) 0 (select `/Game/Spirit/E_ManaType` (`self.ManaType`) :`NewEnumerator0` "/Game/Spirit/Materials/M_Flora.M_Flora" :`NewEnumerator1` "/Game/Spirit/Materials/M_Fauna.M_Fauna" :`NewEnumerator2` "/Game/Spirit/Materials/M_Flood.M_Flood" :`NewEnumerator3` "/Game/Spirit/Materials/M_Ferrous.M_Ferrous" :`NewEnumerator7` "/Game/Spirit/Materials/M_Flare.M_Flare" :`NewEnumerator6` "/Game/Spirit/Materials/M_Frost.M_Frost" :!type "MaterialInterface Object Reference"))
  (set `self.Home` (`self.K2_GetActorLocation`)))

(event `Harvested`
  (set `self.State` "NewEnumerator1")
  (`MovementComponent.StopMovementImmediately` (`self.CharacterMovement`))
  (`PrimitiveComponent.SetCollisionEnabled` (`self.CapsuleComponent`) "NoCollision")
  (`SceneComponent.SetVisibility` (`self.CapsuleComponent`) false true))

(event `Used`
  (params (NewLocation :type "Vector Structure"))
  (`PrimitiveComponent.SetCollisionEnabled` (`self.CapsuleComponent`) "QueryAndPhysics")
  (`SceneComponent.SetVisibility` (`self.CapsuleComponent`) true true)
  (set `self.State` "NewEnumerator2")
  (`KismetSystemLibrary.Delay` 4.0)
  (set `self.State` "NewEnumerator3")
  (`self.Return`))

(event `Return`
  (`|AIMoveTo` self (`self.Home`) null 3.0
    (:`OnSuccess`
      (if (< (`KismetMathLibrary.Vector_DistanceSquared` (`self.Home`) (`self.K2_GetActorLocation`)) 100000.0)
        (set `self.State` "NewEnumerator0")
        (else
          (`PrimitiveComponent.SetCollisionEnabled` (`self.CapsuleComponent`) "NoCollision")
          (`SceneComponent.SetVisibility` (`self.CapsuleComponent`) false true)
          (`KismetSystemLibrary.Delay` 2.0)
          (`self.K2_SetActorLocation` (`self.Home`))
          (`SceneComponent.SetVisibility` (`self.CapsuleComponent`) true true)
          (`PrimitiveComponent.SetCollisionEnabled` (`self.CapsuleComponent`) "QueryAndPhysics")
          (set `self.State` "NewEnumerator0"))))))

(fn `UserConstructionScript`)
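; Fireball projectile for the player's Flare ability that explodes on hit, or expires without exploding after a short lifetime.
; The explosion reveals BlastRadius and line-traces to overlapping components, so cover blocks its effects.
; Exposed targets get Burn, knockback or damage via interfaces, casts and mobility checks; launched physics objects become damaging projectiles through the instigating player.
; On destruction, it passes its location to CastingHand.EndSpecial.
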(event `self.ReceiveBeginPlay`
  (bind _asbp_first_person_character (cast `/Game/Player/BP_FirstPersonCharacter` (`self.GetInstigator` self))
    (:`then`
      (set `self.Player` _asbp_first_person_character))
    (:`CastFailed`
      (`KismetSystemLibrary.PrintString` "Cast failed - player is not BP_FirstPersonCharacter")))
  (`KismetSystemLibrary.Delay` 2.0)
  (`self.K2_DestroyActor`))

(event `self.ReceiveDestroyed`
  (`/Game/Player/BP_Hand.EndSpecial` (`self.Casting Hand`) (`self.K2_GetActorLocation`) null))

(event `self.ReceiveHit`
  (params (MyComp :type "PrimitiveComponent Object Reference") (Other :type "Actor Object Reference") (OtherComp :type "PrimitiveComponent Object Reference") (bSelfMoved :type Boolean) (HitLocation :type "Vector Structure") (HitNormal :type "Vector Structure") (NormalImpulse :type "Vector Structure") (Hit :type "HitResult Structure (by ref)"))
  (`SceneComponent.SetHiddenInGame` (`self.BlastRadius`) false false)
  (`self.Explode`))

(event `Explode`
  (`|ExecutionSequence`
    (:`then_0`
      (for _array_element (`PrimitiveComponent.GetOverlappingComponents` (`self.BlastRadius`))
        (bind _returnvalue (`ActorComponent.GetOwner` _array_element))
        (bind (_outhit _returnvalue_2) (`KismetSystemLibrary.LineTraceSingle` (`self.K2_GetActorLocation`) (`SceneComponent.K2_GetComponentLocation` _array_element) "TraceTypeQuery4" false (`|MakeArray` _returnvalue)))
        (if (not _returnvalue_2)
          (bind _asbpi_elemental (cast `/Game/EnvironmentBPs/ElementInteraction/Interfaces/BPI_Elemental` _returnvalue)
            (:`then`
              (`/Game/EnvironmentBPs/ElementInteraction/Interfaces/BPI_Elemental.Burn` _asbpi_elemental))
            (:`CastFailed`
              _))
          (switch `EComponentMobility` (`SceneComponent.Mobility` _array_element)
            (:`Static`
              (bind _returnvalue_3 (`ActorComponent.GetOwner` _array_element))
              (if (`KismetSystemLibrary.DoesImplementInterface` _returnvalue_3 "/Game/Enemies/BPI_Hittable.BPI_Hittable_C") :!label _label
                (bind _returnvalue_4 (`KismetMathLibrary.Normal` (- (`SceneComponent.K2_GetComponentLocation` _array_element) (`self.K2_GetActorLocation`))))
                (bind _returnvalue_5 (* _returnvalue_4 1000.0))
                (message `/Game/Enemies/BPI_Hittable.TakeDamage` _returnvalue_3 99.0 "NewEnumerator7" _returnvalue_5)))
            (:`Stationary`
              (goto _label))
            (:`Movable`
              (bind _ascharacter (cast `Character` _returnvalue_3)
                (:`then`
                  (`CharacterMovementComponent.AddImpulse` (`Character.CharacterMovement` _ascharacter) _returnvalue_5 true)
                  (bind _asbp_first_person_character (cast `/Game/Player/BP_FirstPersonCharacter` _ascharacter)
                    (:`then`
                      (`/Game/Player/BP_FirstPersonCharacter.TakeDamage` _asbp_first_person_character 0.1)
                      (goto _label))
                    (:`CastFailed`
                      (goto _label))))
                (:`CastFailed`
                  (if (`SceneComponent.IsSimulatingPhysics` _array_element "None")
                    (bind _asprimitive_component (cast `PrimitiveComponent` _array_element)
                      (:`then`
                        (`PrimitiveComponent.AddImpulseAtLocation` _asprimitive_component (* _returnvalue_4 800000.0) (`self.K2_GetActorLocation`) "None")
                        (`/Game/Player/BP_FirstPersonCharacter.MakeProjectileDamaging` (`self.Player`) _asprimitive_component)
                        (goto _label))
                      (:`CastFailed`
                        (goto _label)))))))))))
    (:`then_1`
      (`KismetSystemLibrary.Delay` 0.2)
      (`self.K2_DestroyActor`))))

(fn `UserConstructionScript`)
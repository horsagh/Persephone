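; Ice path ability actor that grows a spline-mesh path from the caster toward where their first-person camera aims.
; StartCast places the actor one step ahead of the caster, then a delayed, self-calling event adds a fixed number of segments.
; Each step re-traces from the camera, so the path follows the live aim.
; New segments get their own spline mesh, and the previous segment's end tangent is updated to join smoothly.
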(event `StartCast`
  (params (Caster :type "/Game/Player/BP_FirstPersonCharacter Object Reference"))
  (bind _output_get (set `self.Caster` Caster))
  (bind _next_point (`self.FindNewSplinePointLocation` (`self.K2_GetActorLocation` _output_get)))
  (`self.K2_SetActorLocation` _next_point)
  (`self.NewNode`))

(event `NewNode`
  (bind _iterations (`self.Iterations`))
  (bind (_location _tangent) (`SplineComponent.GetLocationAndTangentAtSplinePoint` (`self.Spline`) _iterations "Local"))
  (bind (_location_2 _tangent_2) (`SplineComponent.GetLocationAndTangentAtSplinePoint` (`self.Spline`) (+ (`self.Iterations`) 1) "Local"))
  (`KismetSystemLibrary.Delay` 0.3)
  (`|ExecutionSequence`
    (:`then_0`
      ;[1 1 1] Add spline point
      (bind _next_point (`self.FindNewSplinePointLocation` (`SplineComponent.GetLocationAtSplinePoint` (`self.Spline`) (`self.Iterations`) "World")))
      (`SplineComponent.AddSplinePoint` (`self.Spline`) _next_point "World" true)
      ;[1 1 1] Create and position splinemesh
      (bind _returnvalue (`AddComponent|NODE_AddSplineMeshComponent-2`))
      (`KismetArrayLibrary.Array_Add` (`self.SplineMesh`) _returnvalue)
      (`SceneComponent.K2_AttachToComponent` _returnvalue (`self.Spline`) "None" "KeepRelative" "KeepRelative" "KeepRelative" true)
      (`SplineMeshComponent.SetStartAndEnd` (`|GetArrayItem` (`self.SplineMesh`) _iterations) _location _tangent _location_2 _tangent_2 true)
      (if (!= (`self.Iterations`) 0)
        (`SplineMeshComponent.SetEndTangent` (`|GetArrayItem` (`self.SplineMesh`) (- (`self.Iterations`) 1)) _tangent true)))
    (:`then_1`
      ;[1 1 1] Recursion
      (bind _result (`/Engine/EditorBlueprintResources/StandardMacros.IncrementInt` (`self.Iterations`))
        (:`  `
          (if (< _result 7)
            (`self.NewNode`)))))))

(fn `FindNewSplinePointLocation`
  (params (`Previous Point` :type "Vector Structure"))
  (returns (`Next Point` :type "Vector Structure"))
  (locals (PreviousPoint :type "Vector Structure"))
  (bind _firstpersoncamera (`/Game/Player/BP_FirstPersonCharacter.FirstPersonCamera` (`self.Caster`)))
  (bind _returnvalue (`SceneComponent.K2_GetComponentLocation` _firstpersoncamera))
  (bind _returnvalue_2 (+ _returnvalue (* (`SceneComponent.GetForwardVector` _firstpersoncamera) 1000.0)))
  (set `local.PreviousPoint` `Previous Point`)
  (bind (_outhit _returnvalue_3) (`KismetSystemLibrary.LineTraceSingle` :`Start` _returnvalue :`End` _returnvalue_2 :`TraceChannel` "TraceTypeQuery1" :`DrawDebugType` "ForDuration"))
  (return (+ (`local.Previous Point`) (* (`KismetMathLibrary.Normal` (- (`KismetMathLibrary.SelectVector` (`.Location` (`GameplayStatics.BreakHitResult` _outhit)) _returnvalue_2 _returnvalue_3) (`local.PreviousPoint`))) 500.0))))

(fn `UserConstructionScript`)
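; Rock pillar player ability actor that rises on spawn and launches overlapping characters along its up axis.
; BeginPlay eases the Pillar component upward, then after a brief delay zeroes the velocity of characters in LaunchBox and launches them.
; Burn, Freeze and Waterlog events drive an elemental state machine where opposing elements cancel or convert, and freezing a waterlogged pillar destroys it.
; It also stores a Spirit reference, exposed with the state through getters.
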(event `self.ReceiveBeginPlay`
  (bind _returnvalue (`self.GetActorUpVector`))
  (`KismetSystemLibrary.MoveComponentTo` (`self.Pillar`) (0.0 0.0 100.0) (struct) false true)
  (`KismetSystemLibrary.Delay` 0.02)
  (for _array_element (`PrimitiveComponent.GetOverlappingActors` (`self.LaunchBox`) "/Script/Engine.Character")
    (bind _ascharacter (cast `Character` _array_element))
    (bind _charactermovement (`Character.CharacterMovement` _ascharacter))
    (set `MovementComponent.Velocity` (0.0 0.0 0.0) _charactermovement)
    (`Character.LaunchCharacter` _ascharacter (+ (`KismetMathLibrary.ProjectVectorOnToPlane` (`MovementComponent.Velocity` _charactermovement) _returnvalue) (* _returnvalue 1000.0)) true true)))

(event `/Game/EnvironmentBPs/ElementInteraction/Interfaces/BPI_Elemental.Burn`
  (switch `/Game/EnvironmentBPs/ElementInteraction/Interfaces/E_ElementalState` (`self.ElementalState`)
    (:`NewEnumerator0`
      (set `self.ElementalState` "NewEnumerator1"))
    (:`NewEnumerator2`
      (set `self.ElementalState` "NewEnumerator3"))
    (:`NewEnumerator3`
      (set `self.ElementalState` "NewEnumerator0"))))

(event `/Game/EnvironmentBPs/ElementInteraction/Interfaces/BPI_Elemental.Freeze`
  (switch `/Game/EnvironmentBPs/ElementInteraction/Interfaces/E_ElementalState` (`self.ElementalState`)
    (:`NewEnumerator0`
      (set `self.ElementalState` "NewEnumerator2"))
    (:`NewEnumerator1`
      (set `self.ElementalState` "NewEnumerator3"))
    (:`NewEnumerator3`
      (`self.K2_DestroyActor`))))

(event `/Game/EnvironmentBPs/ElementInteraction/Interfaces/BPI_Elemental.Waterlog`
  (switch `/Game/EnvironmentBPs/ElementInteraction/Interfaces/E_ElementalState` (`self.ElementalState`)
    (:`NewEnumerator0`
      (set `self.ElementalState` "NewEnumerator3"))
    (:`NewEnumerator1`
      (set `self.ElementalState` "NewEnumerator0"))))

(event `/Game/EnvironmentBPs/Spirit/BPI_SpiritContainer.SetSpirit`
  (params (NewSpirit :type "/Game/EnvironmentBPs/BP_Spirit Object Reference"))
  (set `self.Spirit` NewSpirit))

(fn `GetElementalState`
  (returns (ElementalState :type "/Game/EnvironmentBPs/ElementInteraction/Interfaces/E_ElementalState Enum"))
  (return (`self.ElementalState`)))

(fn `GetSpirit`
  (returns (Spirit :type "/Game/EnvironmentBPs/BP_Spirit Object Reference"))
  (return (`self.Spirit`)))

(fn `UserConstructionScript`)
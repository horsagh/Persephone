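; BP_Spirit is a harvestable spirit character whose sphere material reflects its mana type.
; Harvesting halts and hides it, disables collision and moves it to world origin.
; Using it sets a new Home, then teleports it there and restores it after delays, tracked by a State enum.
; Containers implementing BPI_SpiritContainer receive the spirit instead of triggering that return; an AIMoveTo walk-home path is left unconnected.
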(event `self.ReceiveBeginPlay`
  (`PrimitiveComponent.SetMaterial` (`self.Sphere`) 0 (select `/Game/EnvironmentBPs/Spirit/E_ManaType` (`self.ManaType`) :`NewEnumerator0` "/Game/EnvironmentBPs/Spirit/Materials/M_Flora.M_Flora" :`NewEnumerator1` "/Game/EnvironmentBPs/Spirit/Materials/M_Fauna.M_Fauna" :`NewEnumerator2` "/Game/EnvironmentBPs/Spirit/Materials/M_Flood.M_Flood" :`NewEnumerator3` "/Game/EnvironmentBPs/Spirit/Materials/M_Ferrous.M_Ferrous" :`NewEnumerator7` "/Game/EnvironmentBPs/Spirit/Materials/M_Flare.M_Flare" :`NewEnumerator6` "/Game/EnvironmentBPs/Spirit/Materials/M_Frost.M_Frost" :!type "MaterialInterface Object Reference"))
  (set `self.Home` (`self.K2_GetActorLocation`)))

(event `Harvested`
  (set `self.State` "NewEnumerator1")
  (`MovementComponent.StopMovementImmediately` (`self.CharacterMovement`))
  (`PrimitiveComponent.SetCollisionEnabled` (`self.CapsuleComponent`) "NoCollision")
  (`SceneComponent.SetVisibility` (`self.CapsuleComponent`) false true)
  (`self.K2_SetActorLocation` (0.0 0.0 0.0)))

(event `Used`
  (params (NewLocation :type "Vector Structure"))
  (set `self.Home` NewLocation)
  (set `self.State` "NewEnumerator2")
  (`self.Return`))

(event `Return`
  (`self.K2_SetActorLocation` (`self.Home`))
  (`KismetSystemLibrary.Delay` 1.5)
  (`PrimitiveComponent.SetCollisionEnabled` (`self.CapsuleComponent`) "QueryAndPhysics")
  (`SceneComponent.SetVisibility` (`self.CapsuleComponent`) true true)
  (`KismetSystemLibrary.Delay` 1.5)
  (set `self.State` "NewEnumerator0"))

(event `UsedContainer`
  (params (Container :type "Actor Object Reference"))
  (bind _returnvalue (`self.K2_GetActorLocation` Container))
  (bind _asbpi_spirit_container (cast `/Game/EnvironmentBPs/Spirit/BPI_SpiritContainer` Container)
    (:`then`
      (set `self.Home` _returnvalue)
      (set `self.State` "NewEnumerator2")
      (`/Game/EnvironmentBPs/Spirit/BPI_SpiritContainer.SetSpirit` _asbpi_spirit_container self)
      (`KismetSystemLibrary.Delay` 2.5)
      (set `self.State` "NewEnumerator0"))
    (:`CastFailed`
      (`self.Used` _returnvalue))))

(fn `UserConstructionScript`)
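; BP_Boulder is an environment boulder that changes elemental state when burned, frozen or waterlogged, showing the current state on a text render each tick.
; Each elemental event switches on the current state, with opposing elements converting it to Waterlogged or Default.
; Freezing a waterlogged boulder swaps its mesh for a physics Geometry Collection, spawns BP_Magnesium and triggers a Chaos master field.
; Burning a waterlogged boulder only prints a delayed explosion placeholder.
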(event `self.ReceiveTick`
  (params (DeltaSeconds :type "Float (single-precision)"))
  (`TextRenderComponent.K2_SetText` (`self.TextRender`) (`KismetTextLibrary.Conv_StringToText` (`|GetEnumeratorNameAsString` (`self.ElementalState`)))))

(event `Spawn Magnesium`
  (bind _geometrycollection (`self.GeometryCollection`))
  (bind _geometrycollection_2 (`self.GeometryCollection`))
  (`ActorComponent.K2_DestroyComponent` (`self.StaticMesh`))
  (`PrimitiveComponent.SetCollisionEnabled` (`self.GeometryCollection`) "QueryAndPhysics")
  (`PrimitiveComponent.SetSimulatePhysics` _geometrycollection_2 true)
  (`SceneComponent.SetHiddenInGame` _geometrycollection_2 false false)
  (`|SpawnActorFromClass` "/Game/EnvironmentBPs/BP_Magnesium.BP_Magnesium_C" (`KismetMathLibrary.Conv_VectorToTransform` (`SceneComponent.K2_GetComponentLocation` _geometrycollection_2)) "Undefined" "OverrideRootScale" null null)
  (`PrimitiveComponent.SetCollisionResponseToChannel` _geometrycollection "ECC_GameTraceChannel4" "ECR_Ignore")
  (bind _returnvalue (`|SpawnActorFromClass` "/Engine/EditorResources/FieldNodes/FS_MasterField.FS_MasterField_C" (`KismetMathLibrary.Conv_VectorToTransform` (`SceneComponent.K2_GetComponentLocation` _geometrycollection)) "Undefined" "OverrideRootScale" null null))
  (set `/Engine/EditorResources/FieldNodes/FS_MasterField.ForceMult` 10.0 _returnvalue)
  (`/Engine/EditorResources/FieldNodes/FS_MasterField.CE_Trigger` _returnvalue))

(event `/Game/EnvironmentBPs/ElementInteraction/Interfaces/BPI_Elemental.Burn`
  (switch `/Game/EnvironmentBPs/ElementInteraction/Interfaces/E_ElementalState` (`self.ElementalState`)
    (:`NewEnumerator0`
      (set `self.ElementalState` "NewEnumerator1"))
    (:`NewEnumerator2`
      (set `self.ElementalState` "NewEnumerator3"))
    (:`NewEnumerator3`
      (`self.Delayed Explosion`))))

(event `/Game/EnvironmentBPs/ElementInteraction/Interfaces/BPI_Elemental.Freeze`
  (switch `/Game/EnvironmentBPs/ElementInteraction/Interfaces/E_ElementalState` (`self.ElementalState`)
    (:`NewEnumerator0`
      (set `self.ElementalState` "NewEnumerator2"))
    (:`NewEnumerator1`
      (set `self.ElementalState` "NewEnumerator3"))
    (:`NewEnumerator3`
      (`KismetSystemLibrary.Delay` 0.05)
      (`self.Spawn Magnesium`))))

(event `Delayed Explosion`
  (`KismetSystemLibrary.PrintString` "sizzle")
  (`KismetSystemLibrary.Delay` 1.0)
  (`KismetSystemLibrary.PrintString` "Boom"))

(event `/Game/EnvironmentBPs/ElementInteraction/Interfaces/BPI_Elemental.Waterlog`
  (switch `/Game/EnvironmentBPs/ElementInteraction/Interfaces/E_ElementalState` (`self.ElementalState`)
    (:`NewEnumerator0`
      (set `self.ElementalState` "NewEnumerator3"))
    (:`NewEnumerator1`
      (set `self.ElementalState` "NewEnumerator0"))))

(fn `GetElementalState`
  (returns (ElementalState :type "/Game/EnvironmentBPs/ElementInteraction/Interfaces/E_ElementalState Enum"))
  (return (`self.ElementalState`)))

(fn `UserConstructionScript`)
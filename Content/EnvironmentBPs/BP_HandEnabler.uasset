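; BP_HandEnabler is a pickup actor that enables the first-person character's right or left hand, chosen by IsRightHand.
; On overlap it registers itself as the character's Zone and shows a right or left mouse button pickup prompt, clearing both when overlap ends.
; Its Pickup event, called from outside this graph, enables the matching hand, refreshes that hand's mana UI and destroys the actor.
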(event `self.ReceiveActorBeginOverlap`
  (params (OtherActor :type "Actor Object Reference"))
  (bind _asbp_first_person_character (cast `/Game/Player/BP_FirstPersonCharacter` OtherActor))
  (set `/Game/Player/BP_FirstPersonCharacter.Zone` self _asbp_first_person_character)
  (`TextBlock.SetText` (`/Game/Player/WBP_FirstPerson.PopUpText` (`/Game/Player/BP_FirstPersonCharacter.UI` _asbp_first_person_character)) (select `bool` (`self.isRightHand`) :`false` "Press LMB to pick up" :`true` "Press RMB to pick up" :!type "Text")))

(event `self.ReceiveActorEndOverlap`
  (params (OtherActor :type "Actor Object Reference"))
  (bind _asbp_first_person_character (cast `/Game/Player/BP_FirstPersonCharacter` OtherActor))
  (set `/Game/Player/BP_FirstPersonCharacter.Zone` null _asbp_first_person_character)
  (`TextBlock.SetText` (`/Game/Player/WBP_FirstPerson.PopUpText` (`/Game/Player/BP_FirstPersonCharacter.UI` _asbp_first_person_character)) ""))

(event `Pickup`
  (params (Character :type "/Game/Player/BP_FirstPersonCharacter Object Reference"))
  (bind _returnvalue (select `bool` (`self.isRightHand`) :`false` (`/Game/Player/BP_FirstPersonCharacter.LeftHand` Character) :`true` (`/Game/Player/BP_FirstPersonCharacter.RightHand` Character)))
  (set `/Game/Player/BP_Hand.isEnabled` true _returnvalue)
  (`/Game/Player/BP_Hand.UpdateManaUI` _returnvalue)
  (`self.K2_DestroyActor`))

(fn `UserConstructionScript`)
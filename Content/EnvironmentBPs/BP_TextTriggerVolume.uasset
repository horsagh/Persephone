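; BP_TextTriggerVolume is a trigger actor that shows timed pop-up text on the player's UI when the first-person character overlaps it.
; The overlap calls the TriggerText dispatcher, bound at BeginPlay to ShowText, which fires once or repeatedly depending on Retriggerable.
; ShowText sets the pop-up text, waits for Duration, then clears it only if unchanged, leaving any different, newer message intact.
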(event `self.ReceiveActorBeginOverlap`
  (params (OtherActor :type "Actor Object Reference"))
  (cast `/Game/Player/BP_FirstPersonCharacter` OtherActor)
  (`self.TriggerText`))

(event `self.ReceiveBeginPlay`
  (add `self.TriggerText` (delegate `ShowText`)))

(event `ShowText`
  (if (`self.Retriggerable`)
    (bind _asbp_first_person_character (cast `/Game/Player/BP_FirstPersonCharacter` (`GameplayStatics.GetPlayerCharacter` 0) :!label _label))
    (bind _popuptext (`/Game/Player/WBP_FirstPerson.PopUpText` (`/Game/Player/BP_FirstPersonCharacter.UI` _asbp_first_person_character)))
    (`TextBlock.SetText` _popuptext (`self.Text`))
    (`KismetSystemLibrary.Delay` (`self.Duration`))
    (if (`KismetTextLibrary.EqualEqual_TextText` (`self.Text`) (`TextBlock.GetText` _popuptext))
      (`TextBlock.SetText` _popuptext ""))
    (elif (not (`self.Triggered`))
      (set `self.Triggered` true)
      (goto _label))))

(fn `UserConstructionScript`)
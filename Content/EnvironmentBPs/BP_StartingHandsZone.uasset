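; A zone actor that sets whether each of the first-person character's hands starts enabled or disabled, for characters overlapping it at game start.
; On the first Tick only, it finds overlapping BP_FirstPersonCharacter actors, applies its RightHandEnabled and LeftHandEnabled flags and refreshes each hand's mana UI.
; It uses a one-shot Tick guarded by HasFired because overlaps are not yet registered during BeginPlay.
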(event `self.ReceiveTick`
  (params (DeltaSeconds :type "Float (single-precision)"))
  (if (not (`self.hasFired`))
    (set `self.hasFired` true)
    (for _array_element (`self.GetOverlappingActors` "/Game/Player/BP_FirstPersonCharacter.BP_FirstPersonCharacter_C")
      (bind _asbp_first_person_character (cast `/Game/Player/BP_FirstPersonCharacter` _array_element))
      (`|ExecutionSequence`
        (:`then_0`
          (bind _righthand (`/Game/Player/BP_FirstPersonCharacter.RightHand` _asbp_first_person_character))
          (set `/Game/Player/BP_Hand.isEnabled` (`self.RightHandEnabled`) _righthand)
          (`/Game/Player/BP_Hand.UpdateManaUI` _righthand))
        (:`then_1`
          (bind _lefthand (`/Game/Player/BP_FirstPersonCharacter.LeftHand` _asbp_first_person_character))
          (set `/Game/Player/BP_Hand.isEnabled` (`self.LeftHandEnabled`) _lefthand)
          (`/Game/Player/BP_Hand.UpdateManaUI` _lefthand))))))

(fn `UserConstructionScript`)
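; Trigger volume that resets the game by opening a level when the first-person character overlaps it.
; The game mode builds the options string from the player and the UseCheckpoint setting, which is passed to an absolute Open Level call.
; A GetLevelName helper is meant to pick the configured LevelName, falling back to the current level when that is None.
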(event `self.ReceiveActorBeginOverlap`
  (params (OtherActor :type "Actor Object Reference"))
  (bind _asbp_first_person_character (cast `/Game/Player/BP_FirstPersonCharacter` OtherActor))
  (bind _asbp_first_person_game_mode (cast `/Game/Player/BP_FirstPersonGameMode` (`GameplayStatics.GetGameMode`)))
  (bind _optionsstring (`/Game/Player/BP_FirstPersonGameMode.MakeOptionsString` _asbp_first_person_game_mode (`self.Use Checkpoint`) _asbp_first_person_character))
  (bind _returnvalue (`GameplayStatics.GetCurrentLevelName` true))
  (`GameplayStatics.OpenLevel` (`self.GetLevelName` _returnvalue) true _optionsstring))

(fn `UserConstructionScript`)
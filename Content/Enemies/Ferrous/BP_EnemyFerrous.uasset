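; Ferrous enemy that moves toward a perceived player and fires a floor-is-lava area attack shortly after BeginPlay.
; The attack gathers the floor mesh underfoot plus overlapping meshes, then line-traces points around itself to place warning decals.
; After a delay, a repeating tick damages other characters inside the AOE sphere standing on those meshes, via BPI_Hittable or the player cast.
; ThrowRock is an empty stub.
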(event `self.ReceiveBeginPlay`
  (`SphereComponent.SetSphereRadius` (`self.FloorIsLavaAOE`) (* (`self.FloorIsLavaHalfRange`) 4.0) true)
  (`KismetSystemLibrary.Delay` 3.0)
  (`self.FloorIsLavaAttack`))

(event `Throw Rock`)

(event `self.AIPerception.OnPerceptionUpdated`
  (params (UpdatedActors :type "Array of Actor Object Reference (by ref)"))
  (for _array_element UpdatedActors
    (bind _asbp_first_person_character (cast `/Game/Player/BP_FirstPersonCharacter` _array_element))
    (`|AIMoveTo` self (0.0 0.0 0.0) _asbp_first_person_character)))

(event `FloorIsLavaAttack`
  (bind _asstatic_mesh_component (cast `StaticMeshComponent` (`.HitComponent` (`GameplayStatics.BreakHitResult` (`.HitResult` (break `FindFloorResult` (`CharacterMovementComponent.CurrentFloor` (`self.CharacterMovement`))))))))
  (`KismetArrayLibrary.Array_Add` (`self.FloorIsLavaEffectedFloor`) _asstatic_mesh_component)
  (`self.ProximityTester` _asstatic_mesh_component)
  (for _array_element (`self.FloorIsLavaLineTracePoints`)
    (for _array_element_2 (`self.FloorIsLavaEffectedFloor`)
      (bind (_returnvalue_x _returnvalue_y _returnvalue_z) (`KismetMathLibrary.BreakVector` (+ (`self.K2_GetActorLocation`) (* _array_element (`self.FloorIsLavaHalfRange`) 2.0))))
      (bind (_hitlocation _hitnormal _bonename _outhit _returnvalue) (`PrimitiveComponent.K2_LineTraceComponent` _array_element_2 (`KismetMathLibrary.MakeVector` _returnvalue_x _returnvalue_y (+ _returnvalue_z (`self.FloorIsLavaHalfRange`))) (`KismetMathLibrary.MakeVector` _returnvalue_x _returnvalue_y (- _returnvalue_z (`self.FloorIsLavaHalfRange`))) false false false))
      (if _returnvalue
        (bind _returnvalue_2 (`GameplayStatics.SpawnDecalAtLocation` "/Game/Assets/DM_FerrousAttack.DM_FerrousAttack" (30.0 500.0 500.0) _hitlocation (struct :`Pitch` 90.0) (+ (* (`self.FloorIsLavaBetweenHitDelay`) (+ (`self.FloorIsLavaHitsMax`) 4)) 0.5)))
        (`DecalComponent.SetDecalMaterial` _returnvalue_2 "/Game/Assets/DM_FerrousAttack.DM_FerrousAttack")
        (`KismetSystemLibrary.Delay` (* (`self.FloorIsLavaBetweenHitDelay`) 3.0))
        (set `self.FloorIsLavaHitsRemaining` (`self.FloorIsLavaHitsMax`))
        (`self.FloorIsLavaDamageTick`)))))

(event `ProximityTester`
  (params (TestOn :type "StaticMeshComponent Object Reference"))
  (for _array_element (`PrimitiveComponent.GetOverlappingComponents` TestOn)
    (bind _asstatic_mesh_component (cast `StaticMeshComponent` _array_element))
    (if (not (`KismetArrayLibrary.Array_Contains` (`self.FloorIsLavaEffectedFloor`) _asstatic_mesh_component))
      (`KismetArrayLibrary.Array_Add` (`self.FloorIsLavaEffectedFloor`) _asstatic_mesh_component))))

(event `FloorIsLavaDamageTick`
  (`|ExecutionSequence`
    (:`then_0`
      (for _array_element (`PrimitiveComponent.GetOverlappingComponents` (`self.FloorIsLavaAOE`))
        (bind _returnvalue (`ActorComponent.GetOwner` _array_element))
        (if (not (== _returnvalue self))
          (bind _ascharacter (cast `Character` _returnvalue))
          (bind _asstatic_mesh_component (cast `StaticMeshComponent` (`.HitComponent` (`GameplayStatics.BreakHitResult` (`.HitResult` (break `FindFloorResult` (`CharacterMovementComponent.CurrentFloor` (`Character.CharacterMovement` _ascharacter))))))))
          (if (`KismetArrayLibrary.Array_Contains` (`self.FloorIsLavaEffectedFloor`) _asstatic_mesh_component)
            (bind _asbpi_hittable (cast `/Game/Enemies/BPI_Hittable` _ascharacter)
              (:`then`
                (`/Game/Enemies/BPI_Hittable.TakeDamage` _asbpi_hittable (`self.FloorIsLavaEnemyDamage`) "NewEnumerator3" (0.0 0.0 1.0)))
              (:`CastFailed`
                (bind _asbp_first_person_character (cast `/Game/Player/BP_FirstPersonCharacter` _ascharacter))
                (`/Game/Player/BP_FirstPersonCharacter.TakeDamage` _asbp_first_person_character (`self.FloorIsLavaPlayerDamage`))))))))
    (:`then_1`
      (bind _result (`/Engine/EditorBlueprintResources/StandardMacros.DecrementInt` (`self.FloorIsLavaHitsRemaining`))
        (:`  `
          (if (> _result 0)
            (`KismetSystemLibrary.Delay` (`self.FloorIsLavaBetweenHitDelay`))
            (`self.FloorIsLavaDamageTick`)))))))

(fn `Use Proximity Tester`
  (params (`Original Mesh` :type "StaticMeshComponent Object Reference"))
  (locals (ComponentsToAdd :type "Array of StaticMeshComponent Object Reference"))
  (for _array_element (`PrimitiveComponent.GetOverlappingComponents` `Original Mesh`)
    (bind _asstatic_mesh_component (cast `StaticMeshComponent` _array_element))
    (if (not (`KismetArrayLibrary.Array_Contains` (`self.FloorIsLavaEffectedFloor`) _asstatic_mesh_component))
      (`KismetArrayLibrary.Array_Add` (`local.ComponentsToAdd`) _asstatic_mesh_component)))
  (`KismetArrayLibrary.Array_Append` (`self.FloorIsLavaEffectedFloor`) (`local.ComponentsToAdd`)))

(fn `UserConstructionScript`
  (`parent.UserConstructionScript`))
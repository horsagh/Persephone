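; Enemy Blueprint with health shown on a text render and a physics-driven death.
; TakeDamage subtracts health when no invulnerability timer is running and stores the hit direction.
; Tick calls Die at zero health, which spawns a skeletal mesh actor copying the mesh and materials, then destroys the enemy.
; The copy simulates physics, ignores Pawn and one custom channel, and gets an impulse along the last hit direction.
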(event `/Game/Enemies/BPI_Hittable.TakeDamage`
  (params (Damage :type Integer) (Type :type "/Game/EnvironmentBPs/Spirit/E_ManaType Enum" :default "NewEnumerator0") (HitForwardVec :type "Vector Structure"))
  (if (<= (`self.InvulnerabilityTimer`) 0.0)
    (bind _output_get (set `self.Health` (- (`self.Health`) Damage)))
    (`TextRenderComponent.K2_SetText` (`self.TextRender`) (`KismetTextLibrary.Conv_IntToText` _output_get))
    (set `self.MostRecentHit` HitForwardVec)))

(event `Die`
  (`self.SetActorEnableCollision` false)
  (bind _returnvalue (`|SpawnActorFromClass` "/Script/Engine.SkeletalMeshActor" (`SceneComponent.K2_GetComponentToWorld` (`self.Mesh`)) "Undefined" "MultiplyWithRoot" null null))
  (bind _skeletalmeshcomponent (`SkeletalMeshActor.SkeletalMeshComponent` _returnvalue))
  (`SkinnedMeshComponent.SetSkinnedAssetAndUpdate` _skeletalmeshcomponent (`SkeletalMeshComponent.SkeletalMeshAsset` (`self.Mesh`)) false)
  (for (_array_element _array_index) (`MeshComponent.GetMaterials` (`self.Mesh`))
    (`PrimitiveComponent.SetMaterial` _skeletalmeshcomponent _array_index _array_element))
  (`PrimitiveComponent.SetCollisionEnabled` _skeletalmeshcomponent "QueryAndPhysics")
  (`PrimitiveComponent.SetCollisionResponseToChannel` _skeletalmeshcomponent "ECC_GameTraceChannel4" "ECR_Ignore")
  (`PrimitiveComponent.SetCollisionResponseToChannel` _skeletalmeshcomponent "ECC_Pawn" "ECR_Ignore")
  (`PrimitiveComponent.SetSimulatePhysics` _skeletalmeshcomponent true)
  (`PrimitiveComponent.AddImpulse` _skeletalmeshcomponent (* (`KismetMathLibrary.Normal` (`self.MostRecentHit`)) 20000.0) "None" false)
  (`self.K2_DestroyActor`))

(event `self.ReceiveTick`
  (params (DeltaSeconds :type "Float (single-precision)"))
  (if (and (<= (`self.Health`) 0.0) (not (`self.Dead`)))
    (`self.Die`)))

(event `self.ReceiveBeginPlay`
  (`TextRenderComponent.K2_SetText` (`self.TextRender`) (`KismetTextLibrary.Conv_IntToText` (`self.Health`))))

(fn `UserConstructionScript`)